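; Player state for the multiplayer main menu that assigns a randomly generated player name on BeginPlay.
; It builds the name by alternating stringified random floats with random picks from the UserNameRandom array.
; The name is applied through SetPlayerName to player controller index 0, rather than to the controller that owns this player state.
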(event EventBeginPlay
  (Class|AdvancedSessionsLibrary|SetPlayerName (Game|GetPlayerController 0) (Utilities|String|Append (Utilities|String|ToString(Float) (Math|Random|RandomFloatinRange 1e+01 9999.0)) (.OutItem (Utilities|Array|Random (Variables|Default|GetUserNameRandom))) (Utilities|String|ToString(Float) (Math|Random|RandomFloatinRange 1e+01 9999.0)) (.OutItem (Utilities|Array|Random (Variables|Default|GetUserNameRandom))))))

(fn ConstructionScript)