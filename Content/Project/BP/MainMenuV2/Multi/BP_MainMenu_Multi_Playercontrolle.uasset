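; Player controller for the multiplayer main menu that creates the menu widget and handles quitting and session destruction.
; It caches the menu game state on BeginPlay.
; An update event, meant to be called by the game mode, asks the game state to send updates to all players.
; A second event passes the game state and a given player state to the widget to refresh session info.
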(event Custom|Create%20Multi%20Main%20Menu
  (bind _returnvalue (UserInterface|CreateWidget "/Game/Project/BP/MainMenuV2/Multi/WBP_MainMenu_Multi.WBP_MainMenu_Multi_C" (Game|GetPlayerController 0)))
  (bind _output_get (Variables|Default|SetWBP_MainMenu_Multi _returnvalue))
  (UserInterface|Viewport|AddtoViewport _output_get 0))

(event Custom|Quit%20Game
  (Game|QuitGame (Game|GetPlayerController 0) "Quit" false))

(event Custom|Destroy%20session
  (|DestroySession (Game|GetPlayerController 0)))

(event Custom|Update%20all%20WBP
  (params (Playerstate :type Array%20of%20Player%20State%20Object%20References))
  ;[1 1 1] Envoie l'instruction update le widget
  (Default|UpdateSessionInfo (Variables|Default|GetWBP_MainMenu_Multi) (Variables|Default|GetGameState) Playerstate))

(event Custom|Server%20Send%20update%20to%20all%20player
  ;[1 1 1] Le gamemode call pour repliqué les info de la gamestate a tout les widget
  (Default|MultiUpdateSend (Variables|Default|GetGameState)))

(event EventBeginPlay
  (bind _asbp_main_menu_multi_gamestate (Utilities|Casting|CastToBP_MainMenu_Multi_Gamestate (Game|GetGameState)))
  (Variables|Default|SetGameState _asbp_main_menu_multi_gamestate))

(fn ConstructionScript)