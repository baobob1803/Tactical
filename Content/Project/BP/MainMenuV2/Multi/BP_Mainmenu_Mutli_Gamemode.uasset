(event EventBeginPlay
  (Utilities|FlowControl|Delay 45.0))

(event EventHandleStartingNewPlayer
  (params (NewPlayer :type Player%20Controller%20Object%20Reference)))

(event EventPostLogin
  (params (NewPlayer :type Player%20Controller%20Object%20Reference))
  (bind _asbp_main_menu_multi_playercontrolle (Utilities|Casting|CastToBP_MainMenu_Multi_Playercontrolle NewPlayer))
  (Utilities|Array|Add (Variables|Default|GetPCList) _asbp_main_menu_multi_playercontrolle)
  (bind _asbp_main_menu_multi_gamestate (Utilities|Casting|CastToBP_MainMenu_Multi_Gamestate (Game|GetGameState)))
  (Variables|Default|SetBp_GameState _asbp_main_menu_multi_gamestate)
  (Utilities|FlowControl|Sequence
    (:then_0
      (Default|CreateMultiMainMenu _asbp_main_menu_multi_playercontrolle))
    (:then_1
      (Default|UpdateSessionCurrentPlayer (Variables|Default|GetBp_GameState) (Utilities|Array|Length (Variables|Default|GetPCList))))
    (:then_2
      (Utilities|FlowControl|Delay 0.5)
      (Default|ServerSendUpdatetoAllPlayer _asbp_main_menu_multi_playercontrolle))
    (:then_3
      (Utilities|FlowControl|Delay 1.5)
      (Default|ServerSendUpdatetoAllPlayer _asbp_main_menu_multi_playercontrolle))))

(event EventOnLogout
  (params (ExitingController :type Controller%20Object%20Reference))
  (bind _pclist (Variables|Default|GetPCList))
  (bind _asbp_main_menu_multi_playercontrolle (Utilities|Casting|CastToBP_MainMenu_Multi_Playercontrolle ExitingController)
    (:then
      (Utilities|Array|RemoveItem _pclist _asbp_main_menu_multi_playercontrolle)
      (Utilities|FlowControl|Sequence
        (:then_0
          (Default|UpdateSessionCurrentPlayer (Variables|Default|GetBp_GameState) (Utilities|Array|Length _pclist)))
        (:then_1
          (Utilities|FlowControl|Delay 0.5)
          (Default|ServerSendUpdatetoAllPlayer (Utilities|Array|Get(acopy) (Variables|Default|GetPCList))))))
    (:CastFailed
      (Development|PrintString "GM Cast failed"))))

(fn ConstructionScript)