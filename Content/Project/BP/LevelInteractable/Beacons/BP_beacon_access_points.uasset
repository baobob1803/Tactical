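; Beacon access point that hands out a player's bought weapon when a master character walks into its sphere.
; On overlap it looks up the linked beacon's bought-weapon map, keyed by the net index of the local viewing player controller, then spawns the weapon and clears that entry.
; Spawning resolves the weapon name to a class through DT_weapon_class_match, places it at SpawnerPosition and initializes its weapon data.
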(event OnComponentBeginOverlap(Sphere)
  (params (OverlappedComponent :type Primitive%20Component%20Object%20Reference) (OtherActor :type Actor%20Object%20Reference) (OtherComp :type Primitive%20Component%20Object%20Reference) (OtherBodyIndex :type Integer) (bFromSweep :type Boolean) (SweepResult :type Hit%20Result%20Structure%20%28by%20ref%29))
  (bind _beacon_ref (Variables|Default|GetBeacon%20Ref))
  (bind _dict_of_bought_weapons (Variables|/Game/Project/BP/LevelInteractable/Beacons/BP_Weapon_Beacon.BP_Weapon_Beacon_C|GetDict%20of%20bought%20weapons _beacon_ref))
  (if (Class|GameplayStatics|ObjectIsA OtherActor "/Game/Project/BP/GameManagement/Match/BP_Master_Character.BP_Master_Character_C")
    (bind _asbp_master_character (Utilities|Casting|CastToBP_Master_Character OtherActor))
    (if (.ReturnValue (Utilities|Map|Find _dict_of_bought_weapons (Class|AdvancedSessionsLibrary|GetNetPlayerIndex (Pawn|GetLocalViewingPlayerController _asbp_master_character))))
      (CallFunction|SpawnWeapon (.Value (Utilities|Map|Find _dict_of_bought_weapons (Class|AdvancedSessionsLibrary|GetNetPlayerIndex (Pawn|GetLocalViewingPlayerController _asbp_master_character)))))
      (Utilities|Map|Remove _dict_of_bought_weapons (Class|AdvancedSessionsLibrary|GetNetPlayerIndex (Pawn|GetLocalViewingPlayerController _asbp_master_character))))))

(fn ConstructionScript)

(fn SpawnWeapon
  (params (Weapon%20name :type String))
  (bind _spawner_position (Variables|Default|GetSpawner%20position))
  (bind _returnvalue (Transformation|GetWorldTransform _spawner_position))
  (bind _returnvalue_2 (Utilities|GetDataTableRow "/Game/Project/BP/Data/BDD/DT_weapon_class_match.DT_weapon_class_match" (Utilities|String|StringToName Weapon%20name))
    (:then
      (bind _returnvalue_3 (Game|SpawnActorfromClass (Utilities|Struct|BreakS_weapon_class_match _returnvalue_2) (Math|Transform|MakeTransform (.location _returnvalue) (.rotation _returnvalue) "1.000000,1.000000,1.000000") "AdjustIfPossibleButAlwaysSpawn" "MultiplyWithRoot" 0 0))
      (Default|InitializeWeaponData _returnvalue_3 Weapon%20name))
    (:RowNotFound
      (Development|PrintString "Can't purchase weapon because row not found in data table (WBP_weapon_shop)"))))