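; Soft box level interactable that acts as a damageable target for weapon shots, currently as a debug-level implementation.
; DamageActor takes the ammo name and penetration advancement, but only prints a debug message and returns a constant 1 regardless of either.
; Unconnected draft graphs look up ammo penetration levels in a data table, noted for possible per-box shot-blocking behavior.
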(event EventBeginPlay)

(event Collision|EventActorBeginOverlap
  (params (OtherActor :type Actor%20Object%20Reference)))

(event EventTick
  (params (DeltaSeconds :type Float%20%28single-precision%29)))

(fn ConstructionScript)

(fn DamageActor
  (params (Ammo%20name :type String) (Penetration%20advancement :type Integer))
  (Development|PrintString "Damaged" true true "(R=0.055018,G=1.000000,B=0.000000,A=1.000000)")
  (return 1))