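; Player state for the multiplayer main menu lobby that holds the player's name and team and saves them to disk.
; Shortly after BeginPlay, it sets the name from the Steam persona of player controller 0, or from PlayerId without Steam.
; Save_Lobby_Info writes name, team and lobby player count through one BP_Main_Menu_Save object into three slots, each keyed by a prefix plus GetPlayerName.
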(event Custom|Save_Lobby_Info
  (bind _returnvalue (SaveGame|CreateSaveGameObject "/Game/Project/BP/GameManagement/MainMenu/Multi/BP_Main_Menu_Save.BP_Main_Menu_Save_C"))
  (Variables|/Game/Project/BP/GameManagement/MainMenu/Multi/BP_Main_Menu_Save.BP_Main_Menu_Save_C|SetPseudo _returnvalue (Variables|Default|GetName))
  (SaveGame|SaveGametoSlot _returnvalue (Utilities|String|Append "Name" (PlayerState|GetPlayerName)))
  (Variables|/Game/Project/BP/GameManagement/MainMenu/Multi/BP_Main_Menu_Save.BP_Main_Menu_Save_C|SetCurrentTeam _returnvalue (Variables|Default|GetCurrentTeamJoin))
  (SaveGame|SaveGametoSlot _returnvalue (Utilities|String|Append "TeamJoined" (PlayerState|GetPlayerName)))
  (Variables|/Game/Project/BP/GameManagement/MainMenu/Multi/BP_Main_Menu_Save.BP_Main_Menu_Save_C|SetLobbyPlayerCount _returnvalue (Utilities|Array|Length (Variables|/Script/Engine.GameStateBase|GetPlayerArray (.AsBP%20Main%20Menu%20Multi%20Gamestate (Utilities|Casting|CastToBP_MainMenu_Multi_Gamestate (Game|GetGameState))))))
  (SaveGame|SaveGametoSlot _returnvalue (Utilities|String|Append "LobbyCount" (PlayerState|GetPlayerName)))
  (Development|PrintString "Saved Info"))

(event EventBeginPlay
  (Utilities|FlowControl|Delay 0.2)
  (if (Class|AdvancedSessionsLibrary|HasOnlineSubsystem "STEAM")
    (bind _returnvalue (Class|AdvancedSteamFriendsLibrary|GetSteamPersonaName (Class|AdvancedSessionsLibrary|GetUniqueNetID (Game|GetPlayerController 0))))
    (Variables|Default|SetName (Utilities|String|StringToName _returnvalue))
    (else
      (Variables|Default|SetName (Utilities|String|StringToName (Utilities|String|ToString(Integer) (Variables|Default|GetPlayerId)))))))

(fn ConstructionScript)