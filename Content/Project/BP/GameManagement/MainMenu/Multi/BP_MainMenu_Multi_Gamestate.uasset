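; Game state for the multiplayer main menu lobby, tracking the session player count and attack and defense team sizes.
; Team balancing sends a player to the smaller team, favoring attack on a tie.
; Joining increments that team's count, records the team on the PlayerState and triggers a Serv-to-Multi event chain that refreshes lobby info through each controller in PlayerArray.
; A separate event requests a player count text update through the first player controller.
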(event Custom|Update%20Session%20Current%20Player
  (params (CurrentPlayer :type Integer))
  ;[1 1 1] (Server) Update Player Session Count
  (Variables|Default|SetCurrentPlayer CurrentPlayer))

(event Custom|Update%20Current%20player%20Number
  ;[1 1 1] Envoie cette information a tout les joueurs dans le server (Update le current player text)
  (bind _asbp_main_menu_multi_playercontrolle (Utilities|Casting|CastToBP_MainMenu_Multi_Playercontrolle (Game|GetPlayerController 0)))
  (Default|ServUpdateCurrentPlayerText _asbp_main_menu_multi_playercontrolle))

(event Custom|Serv_Request_Update_WBP_Lobby
  (CallFunction|MultiRequestUpdateWBPLobby))

(event Custom|Join_Attack_Team
  (params (Playercontroller :type BP%20Main%20Menu%20Multi%20Playercontrolle%20Object%20Reference))
  (Variables|Default|SetNumAttackTeam (+ (Variables|Default|GetNumAttackTeam) 1))
  (Variables|/Game/Project/BP/GameManagement/MainMenu/Multi/BP_MainMenu_Multi_Playerstate.BP_MainMenu_Multi_Playerstate_C|SetCurrentTeamJoin (.AsBP%20Main%20Menu%20Multi%20Playerstate (Utilities|Casting|CastToBP_MainMenu_Multi_Playerstate (Variables|/Script/Engine.Controller|GetPlayerState Playercontroller))) 0)
  (CallFunction|ServRequestUpdateWBPLobby))

(event Custom|Join_Defense_Team
  (params (Playercontroller :type BP%20Main%20Menu%20Multi%20Playercontrolle%20Object%20Reference))
  (Variables|Default|SetNumDefenderTeam (+ (Variables|Default|GetNumDefenderTeam) 1))
  (Variables|/Game/Project/BP/GameManagement/MainMenu/Multi/BP_MainMenu_Multi_Playerstate.BP_MainMenu_Multi_Playerstate_C|SetCurrentTeamJoin (.AsBP%20Main%20Menu%20Multi%20Playerstate (Utilities|Casting|CastToBP_MainMenu_Multi_Playerstate (Variables|/Script/Engine.Controller|GetPlayerState Playercontroller))) 1)
  (CallFunction|ServRequestUpdateWBPLobby))

(event Custom|CheckTeamBalance&joinLowest
  (params (PlayerController :type BP%20Main%20Menu%20Multi%20Playercontrolle%20Object%20Reference))
  (Math|Integer|CompareInt (Variables|Default|GetNumAttackTeam) (Variables|Default|GetNumDefenderTeam)
    (:>
      (CallFunction|JoinDefenseTeam PlayerController))
    (:==
      (CallFunction|JoinAttackTeam PlayerController :!label _label))
    (:<
      (goto _label))))

(event Custom|Multi_Request_Update_WBP_Lobby
  (bind _array_element (Utilities|Array|ForEachLoopwithBreak (Variables|Default|GetPlayerArray))
    (:LoopBody
      (bind _asbp_main_menu_multi_playercontrolle (Utilities|Casting|CastToBP_MainMenu_Multi_Playercontrolle (Game|GetPlayerController _array_element)))
      (Default|UpdateWBPLobbyInfo _asbp_main_menu_multi_playercontrolle))))

(fn ConstructionScript)