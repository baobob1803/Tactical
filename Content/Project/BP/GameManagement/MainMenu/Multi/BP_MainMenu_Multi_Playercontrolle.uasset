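; Player controller for the multiplayer main menu: it creates the lobby widget and handles team switching, session destruction and quitting.
; SwitchTeamRequest flips the player state's team, calls the game state's join function, then requests a lobby update after a short delay.
; That request, also bound to the P key, goes through the game state.
; Update_WBP_LobbyInfo rebuilds the attack and defense lists from PlayerArray and refreshes the player count.
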(event Custom|Create%20Multi%20Main%20Menu
  (bind _returnvalue (UserInterface|CreateWidget "/Game/Project/BP/WBP/MainMenu/Multi/WBP_MainMenu_Multi.WBP_MainMenu_Multi_C" (Game|GetPlayerController 0)))
  (bind _output_get (Variables|Default|SetWBP_MainMenu_Multi _returnvalue))
  (UserInterface|Viewport|AddtoViewport _output_get 0))

(event Custom|Quit%20Game
  (Game|QuitGame (Game|GetPlayerController 0) "Quit" false))

(event Custom|Destroy%20session
  (|DestroySession (Game|GetPlayerController 0)))

(event Custom|Update_WBP_LobbyInfo
  (bind _wbp_mainmenu_multi (Variables|Default|GetWBP_MainMenu_Multi))
  ;[1 1 1] Update des informations du lobby
  (Widget|Panel|ClearChildren (Variables|/Game/Project/BP/WBP/MainMenu/Multi/WBP_MainMenu_Multi.WBP_MainMenu_Multi_C|GetScrollBox_Attack_List (Variables|Default|GetWBP_MainMenu_Multi)))
  (CallFunction|UpdateCurrentPlayerNumber)
  (bind _array_element (Utilities|Array|ForEachLoopwithBreak (Variables|/Script/Engine.GameStateBase|GetPlayerArray (Variables|Default|GetGameState)))
    (:LoopBody
      (if (== (Variables|/Game/Project/BP/GameManagement/MainMenu/Multi/BP_MainMenu_Multi_Playerstate.BP_MainMenu_Multi_Playerstate_C|GetCurrentTeamJoin (.AsBP%20Main%20Menu%20Multi%20Playerstate (Utilities|Casting|CastToBP_MainMenu_Multi_Playerstate _array_element))) 0)
        (bind _returnvalue (UserInterface|CreateWidget "/Game/Project/BP/WBP/MainMenu/Multi/WBP_Player_Lobby_Info.WBP_Player_Lobby_Info_C" (Game|GetPlayerController 0) (Utilities|Text|ToText(Name) (Variables|/Game/Project/BP/GameManagement/MainMenu/Multi/BP_MainMenu_Multi_Playerstate.BP_MainMenu_Multi_Playerstate_C|GetName (.AsBP%20Main%20Menu%20Multi%20Playerstate (Utilities|Casting|CastToBP_MainMenu_Multi_Playerstate _array_element))))))
        (Widget|Panel|AddChild (Variables|/Game/Project/BP/WBP/MainMenu/Multi/WBP_MainMenu_Multi.WBP_MainMenu_Multi_C|GetScrollBox_Attack_List _wbp_mainmenu_multi) _returnvalue)
        (else
          (bind _returnvalue_2 (UserInterface|CreateWidget "/Game/Project/BP/WBP/MainMenu/Multi/WBP_Player_Lobby_Info.WBP_Player_Lobby_Info_C" (Game|GetPlayerController 0) (Utilities|Text|ToText(Name) (Variables|/Game/Project/BP/GameManagement/MainMenu/Multi/BP_MainMenu_Multi_Playerstate.BP_MainMenu_Multi_Playerstate_C|GetName (.AsBP%20Main%20Menu%20Multi%20Playerstate (Utilities|Casting|CastToBP_MainMenu_Multi_Playerstate _array_element))))))
          (Widget|Panel|AddChild (Variables|/Game/Project/BP/WBP/MainMenu/Multi/WBP_MainMenu_Multi.WBP_MainMenu_Multi_C|GetScrollBox_Defense_List _wbp_mainmenu_multi) _returnvalue_2))))))

(event Custom|Serv_Request_Send%20all%20_Update
  ;[1 1 1] Update des informations du lobby
  (Default|ServRequestUpdateWBPLobby (Variables|Default|GetGameState))
  (Development|PrintString "update Lobby Info"))

(event Custom|SwitchTeamRequest
  (bind _self self)
  (bind _gamestate (Variables|Default|GetGameState))
  (bind _playerstate (Variables|GetPlayerState))
  (bind _asbp_main_menu_multi_playerstate (Utilities|Casting|CastToBP_MainMenu_Multi_Playerstate _playerstate))
  (if (== (Variables|/Game/Project/BP/GameManagement/MainMenu/Multi/BP_MainMenu_Multi_Playerstate.BP_MainMenu_Multi_Playerstate_C|GetCurrentTeamJoin _asbp_main_menu_multi_playerstate) 0)
    (Variables|/Game/Project/BP/GameManagement/MainMenu/Multi/BP_MainMenu_Multi_Playerstate.BP_MainMenu_Multi_Playerstate_C|SetCurrentTeamJoin _asbp_main_menu_multi_playerstate 1)
    (Default|JoinDefenseTeam _gamestate _self)
    (else
      (Variables|/Game/Project/BP/GameManagement/MainMenu/Multi/BP_MainMenu_Multi_Playerstate.BP_MainMenu_Multi_Playerstate_C|SetCurrentTeamJoin _asbp_main_menu_multi_playerstate 0)
      (Default|JoinAttackTeam _gamestate _self)))
  (Utilities|FlowControl|Delay 0.5)
  (CallFunction|ServRequestSendAllUpdate))

(event Custom|Update%20Current%20Player%20Number
  (Rendering|Components|TextRender|SetText (Variables|/Game/Project/BP/WBP/MainMenu/Multi/WBP_MainMenu_Multi.WBP_MainMenu_Multi_C|GetTextBlock_Playernumber (Variables|Default|GetWBP_MainMenu_Multi)) (Utilities|Text|ToText(String) (Utilities|String|Append "Player Number : " (Utilities|String|ToString(Integer) (Variables|/Game/Project/BP/GameManagement/MainMenu/Multi/BP_MainMenu_Multi_Gamestate.BP_MainMenu_Multi_Gamestate_C|GetCurrentPlayer (Variables|Default|GetGameState))) "/" "10"))))

(event EventBeginPlay
  (bind _asbp_main_menu_multi_gamestate (Utilities|Casting|CastToBP_MainMenu_Multi_Gamestate (Game|GetGameState)))
  (Variables|Default|SetGameState _asbp_main_menu_multi_gamestate))

(event Input|KeyboardEvents|P
  (params (Key :type Key%20Structure :default "None"))
  ;[1 1 1] Update des informations du lobby
  (:Pressed
    (CallFunction|ServRequestSendAllUpdate)))

(fn ConstructionScript)