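; Game mode for the multiplayer main menu that manages players joining and leaving.
; On login it stores the controller in PCList, creates its menu, updates the game state's player count and calls its lowest-team balancing.
; After short delays, the joining controller, or the first remaining one after a logout, requests a send-all update from the server.
; HandleStartingNewPlayer is overridden empty, skipping default player start handling.
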(event EventHandleStartingNewPlayer
  (params (NewPlayer :type Player%20Controller%20Object%20Reference)))

(event EventPostLogin
  (params (NewPlayer :type Player%20Controller%20Object%20Reference))
  (bind _asbp_main_menu_multi_playercontrolle (Utilities|Casting|CastToBP_MainMenu_Multi_Playercontrolle NewPlayer))
  (Utilities|Array|Add (Variables|Default|GetPCList) _asbp_main_menu_multi_playercontrolle)
  (bind _asbp_main_menu_multi_gamestate (Utilities|Casting|CastToBP_MainMenu_Multi_Gamestate (Game|GetGameState)))
  (Variables|Default|SetBp_GameState _asbp_main_menu_multi_gamestate)
  (Default|CreateMultiMainMenu _asbp_main_menu_multi_playercontrolle)
  (Utilities|FlowControl|Delay 0.5)
  (Default|UpdateCurrentPlayerNumber (Variables|Default|GetBp_GameState) (Utilities|Array|Length (Variables|Default|GetPCList)))
  (Default|CheckTeamBalance&joinLowest (Variables|Default|GetBp_GameState) _asbp_main_menu_multi_playercontrolle)
  (Utilities|FlowControl|Delay 1.0)
  (Default|ServRequestSendAllUpdate _asbp_main_menu_multi_playercontrolle))

(event EventOnLogout
  (params (ExitingController :type Controller%20Object%20Reference))
  (bind _pclist (Variables|Default|GetPCList))
  (bind _asbp_main_menu_multi_playercontrolle (Utilities|Casting|CastToBP_MainMenu_Multi_Playercontrolle ExitingController)
    (:then
      (Utilities|Array|RemoveItem _pclist _asbp_main_menu_multi_playercontrolle)
      (Utilities|FlowControl|Delay 1.0)
      (Default|ServRequestSendAllUpdate (Utilities|Array|Get(acopy) _pclist))
      (Default|UpdateCurrentPlayerNumber (Variables|Default|GetBp_GameState) (Utilities|Array|Length _pclist)))
    (:CastFailed
      (Development|PrintString "GM Cast failed"))))

(fn ConstructionScript)