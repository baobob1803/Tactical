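; Player controller for the solo main menu, which handles showing the menu, quitting and hosting a multiplayer session.
; BeginPlay creates the solo menu widget and adds it to the viewport.
; CreateServer creates an Advanced Session tagged with a custom string setting and, on success, opens the multiplayer menu level as a listen server.
; LeaveGame quits the game.
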(event Custom|Create%20Server
  (bind _extrasettings (Class|AdvancedSessionsLibrary|GetExtraSettings))
  (bind _modifiedsettingsarray (Class|AdvancedSessionsLibrary|AddorModifyExtraSettings _extrasettings (Utilities|Array|MakeArray (Class|AdvancedSessionsLibrary|MakeLiteralSessionPropertyString "FPSmulti" "TestMap"))))
  (|AdvancedSession _modifiedsettingsarray self 10 0 false true false true true true false false false true false true
    (:OnSuccess
      (Game|OpenLevel(byName) "Main_Menu_Multi" true "?listen"))))

(event Custom|Leave%20Game
  (Game|QuitGame self "Quit" false))

(event Custom|Create%20Solo%20Main%20Menu
  (bind _returnvalue (UserInterface|CreateWidget "/Game/Project/BP/WBP/MainMenu/Solo/WBP_MainMenu_Solo.WBP_MainMenu_Solo_C" self))
  (UserInterface|Viewport|AddtoViewport _returnvalue 0))

(event EventBeginPlay
  (CallFunction|CreateSoloMainMenu))

(fn ConstructionScript)