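; Player controller for the in-match phase, handling the preparation HUD and character spawning.
; On BeginPlay the local controller creates the preparation HUD, then asks BP_GM_InMatch to send HUD init info.
; Events switch the HUD to skill selection with a timer, or spawn and possess a BP_Master_Character at a given transform.
; A debug key prints the player state's HUD-initialise value; team-label and spawn-request logic is left unconnected.
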(event Custom|Ow
  ;[1 1 1] Debug
  (bind _asbp_ps_in_match (Utilities|Casting|CastToBP_PS_InMatch (Variables|GetPlayerState)))
  (Development|PrintString (Utilities|String|ToString(Boolean) (Variables|/Game/Project/BP/GameManagement/Match/BP_PS_InMatch.BP_PS_InMatch_C|GetHUDInitialise _asbp_ps_in_match))))

(event Custom|Start_Skill_Selection
  (bind _hud_preparation (Variables|Default|GetHUD_Preparation))
  (Variables|/Script/UMG.WidgetSwitcher|SetActiveWidgetIndex (Variables|/Game/Project/BP/WBP/Match/PreSquad/WBP_PrepareHUD.WBP_PrepareHUD_C|GetWidgetSwitcher_46 _hud_preparation) 1)
  (Default|LaunchTimer (Variables|/Game/Project/BP/WBP/Match/PreSquad/WBP_SquadPrepare.WBP_SquadPrepare_C|GetWBP_Timer (Variables|/Game/Project/BP/WBP/Match/PreSquad/WBP_PrepareHUD.WBP_PrepareHUD_C|GetWBP_SquadPrepare _hud_preparation))))

(event Custom|Spawn%20Character
  (params (Transform :type Transform))
  (bind _returnvalue (Game|SpawnActorfromClass "/Game/Project/BP/GameManagement/Match/BP_Master_Character.BP_Master_Character_C" Transform "Undefined" "MultiplyWithRoot" self 0))
  (Pawn|Possess _returnvalue))

(event Custom|Serv
  (bind _asbp_gm_in_match (Utilities|Casting|CastToBP_GM_InMatch (Game|GetGameMode)))
  (Default|SendHudInitInfo _asbp_gm_in_match))

(event EventBeginPlay
  (if (Pawn|IsLocalPlayerController)
    (bind _returnvalue (UserInterface|CreateWidget "/Game/Project/BP/WBP/Match/PreSquad/WBP_PrepareHUD.WBP_PrepareHUD_C" (Game|GetPlayerController 0)))
    (bind _output_get (Variables|Default|SetHUD_Preparation _returnvalue))
    (UserInterface|Viewport|AddtoViewport _output_get 0)
    (CallFunction|Serv)))

(event Input|KeyboardEvents|P
  (params (Key :type Key%20Structure :default "None"))
  ;[1 1 1] Debug
  (:Pressed
    (CallFunction|Ow)))

(fn ConstructionScript)

(fn TeamJoin
  (params (TeamJoin :type Integer))
  (if (== TeamJoin 0)
    (return "Team : Attack")
    (else
      (return "Team : Defense"))))