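; In-match game mode that tracks joining player controllers and picks where their characters spawn.
; On login it stores each BP_PC_InMatch in a list, then after a short delay passes that list to BP_GS_InMatch for a total count check.
; The construction script caches every BP_PlayerSpawnPoint.
; Spawn requests send a random cached point's transform back to the controller, which spawns the character, with no occupancy check.
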(event Custom|Get%20Character%20Spawn%20Transform
  (params (Target%20PC :type BP%20PC%20in%20Match%20Object%20Reference))
  (bind _all_spawn_point (Variables|Default|GetAll%20Spawn%20Point))
  ;[1 1 1] Send le transform au PC pour spawn le chara
  (Default|SpawnCharacter Target%20PC (Transformation|GetActorTransform (Utilities|Array|Get(acopy) _all_spawn_point (Math|Random|RandomIntegerinRange 0 (- (Utilities|Array|Length _all_spawn_point) 1))))))

(event EventPostLogin
  (params (NewPlayer :type Player%20Controller%20Object%20Reference))
  (bind _asbp_pc_in_match (Utilities|Casting|CastToBP_PC_InMatch NewPlayer))
  (Utilities|Array|Add (Variables|Default|GetPC_list) _asbp_pc_in_match)
  (bind _asbp_gs_in_match (Utilities|Casting|CastToBP_GS_InMatch (Game|GetGameState)))
  (bind _output_get (Variables|Default|SetBP_GameState _asbp_gs_in_match))
  (Utilities|FlowControl|Delay 1.0)
  (Default|CheckTotalCount _output_get (Variables|Default|GetPC_list)))

(fn ConstructionScript
  (bind _outactors (Actor|GetAllActorsOfClass "/Game/Project/BP/GameManagement/Match/BP_PlayerSpawnPoint.BP_PlayerSpawnPoint_C"))
  (Variables|Default|SetAll%20Spawn%20Point _outactors))