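; In-match player state that restores a player's lobby data when it begins play.
; A one-shot BeginPlay sequence checks three save slots, each keyed by a prefix plus the player name, and loads them as BP_Main_Menu_Save objects.
; It copies the display name (Pseudo), the current team and the lobby player count into its own variables, skipping any missing slot.
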(event EventBeginPlay
  (bind _returnvalue (PlayerState|GetPlayerName))
  (bind _returnvalue_2 (PlayerState|GetPlayerName))
  (bind _returnvalue_3 (PlayerState|GetPlayerName))
  (bind _returnvalue_4 (Utilities|String|Append "LobbyCount" _returnvalue_3))
  (bind _returnvalue_5 (Utilities|String|Append "Name" _returnvalue_2))
  (bind _returnvalue_6 (Utilities|String|Append "TeamJoined" _returnvalue))
  (Utilities|FlowControl|DoOnce false
    (:Completed
      (Utilities|FlowControl|Sequence
        (:then_0
          (bind _returnvalue_7 (SaveGame|DoesSaveGameExist _returnvalue_5))
          (if _returnvalue_7
            (bind _returnvalue_8 (SaveGame|LoadGamefromSlot _returnvalue_5))
            (bind _asbp_main_menu_save (Utilities|Casting|CastToBP_Main_Menu_Save _returnvalue_8))
            (Variables|Default|SetPseudo (Variables|/Game/Project/BP/GameManagement/MainMenu/Multi/BP_Main_Menu_Save.BP_Main_Menu_Save_C|GetPseudo _asbp_main_menu_save))))
        (:then_1
          (bind _returnvalue_9 (SaveGame|DoesSaveGameExist _returnvalue_6))
          (if _returnvalue_9
            (bind _returnvalue_10 (SaveGame|LoadGamefromSlot _returnvalue_6))
            (bind _asbp_main_menu_save_2 (Utilities|Casting|CastToBP_Main_Menu_Save _returnvalue_10))
            (Variables|Default|SetCurrent%20Team (Variables|/Game/Project/BP/GameManagement/MainMenu/Multi/BP_Main_Menu_Save.BP_Main_Menu_Save_C|GetCurrentTeam _asbp_main_menu_save_2))))
        (:then_2
          (bind _returnvalue_11 (SaveGame|DoesSaveGameExist _returnvalue_4))
          (if _returnvalue_11
            (bind _returnvalue_12 (SaveGame|LoadGamefromSlot _returnvalue_4))
            (bind _asbp_main_menu_save_3 (Utilities|Casting|CastToBP_Main_Menu_Save _returnvalue_12))
            (Variables|Default|SetLobbyCount (Variables|/Game/Project/BP/GameManagement/MainMenu/Multi/BP_Main_Menu_Save.BP_Main_Menu_Save_C|GetLobbyPlayerCount _asbp_main_menu_save_3))))))))

(fn ConstructionScript)