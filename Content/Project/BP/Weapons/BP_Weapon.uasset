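; Weapon actor that a BP_Master_Character picks up on overlap, disabling collision, snapping to the character's weapon storage point and passing itself to RetrieveWeapon.
; InitializeWeaponData fills its stats from a data table row by name, mapping category to a type enum and scaling reserve ammo by magazine size.
; UpdateWeaponData copies those stats, including current magazine count, from another weapon instance.
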(event Collision|EventActorBeginOverlap
  (params (OtherActor :type Actor%20Object%20Reference))
  (bind _self self)
  (bind _asbp_master_character (Utilities|Casting|CastToBP_Master_Character OtherActor))
  (Collision|SetCollisionEnabled (Variables|Default|GetCollision) "NoCollision")
  (Transformation|AttachComponentToComponent _self (Variables|/Game/Project/BP/GameManagement/Match/BP_Master_Character.BP_Master_Character_C|Getweaponstoragepoint _asbp_master_character) "None" "SnapToTarget" "SnapToTarget" "KeepRelative" true)
  (Default|RetrieveWeapon _asbp_master_character _self))

(fn ConstructionScript)

(fn InitializeWeaponData
  (params (Weapon%20Name :type String))
  (bind _returnvalue (Utilities|GetDataTableRow "/Game/Project/BP/Data/BDD/Proto_weapon_details_-_Weapon_data_export__2_.Proto_weapon_details_-_Weapon_data_export__2_" (Utilities|String|StringToName Weapon%20Name))
    (:then
      (Utilities|FlowControl|Sequence
        (:then_0
          (Variables|WeaponStats|SetWeapon%20name (.Name (Utilities|Struct|BreakS_weapon_data _returnvalue))))
        (:then_1
          (bind _output_get (Variables|WeaponStats|SetCategory (.Category (Utilities|Struct|BreakS_weapon_data _returnvalue))))
          (switch Utilities|FlowControl|Switch|SwitchonE_weapon_category _output_get
            (:NewEnumerator5
              (Variables|WeaponStats|SetType "NewEnumerator0"))
            (:NewEnumerator0
              (Variables|WeaponStats|SetType "NewEnumerator2"))
            (:NewEnumerator1
              (Variables|WeaponStats|SetType "NewEnumerator1" :!label _label))
            (:NewEnumerator2
              (goto _label))
            (:NewEnumerator3
              (goto _label))
            (:NewEnumerator4
              (goto _label))))
        (:then_2
          (Variables|WeaponStats|SetCost (.Cost (Utilities|Struct|BreakS_weapon_data _returnvalue))))
        (:then_3
          (bind _output_get_2 (Variables|WeaponStats|SetMag%20Size (.MagSize (Utilities|Struct|BreakS_weapon_data _returnvalue))))
          (Variables|WeaponStats|SetCurrentMagValue _output_get_2))
        (:then_4
          (Variables|WeaponStats|SetReload%20time (.ReloadTime (Utilities|Struct|BreakS_weapon_data _returnvalue))))
        (:then_5
          (bind _output_get_3 (Variables|WeaponStats|SetAdditional%20ammo (* (.Additionalammo (Utilities|Struct|BreakS_weapon_data _returnvalue)) (Variables|WeaponStats|GetMag%20Size))))
          (Development|PrintString (Utilities|String|ToString(Integer) _output_get_3) true true "(R=0.000000,G=1.000000,B=0.282915,A=1.000000)"))
        (:then_6
          (Variables|WeaponStats|SetPrimary%20Ammo (.P_ammo (Utilities|Struct|BreakS_weapon_data _returnvalue))))
        (:then_7
          (Variables|WeaponStats|SetSecondary%20Ammo (.S_ammo (Utilities|Struct|BreakS_weapon_data _returnvalue))))))))

(fn UpdateWeaponData
  (params (Weapon%20to%20copy :type BP%20Weapon%20Object%20Reference))
  (Utilities|FlowControl|Sequence
    (:then_0
      (Variables|WeaponStats|SetWeapon%20name (Variables|BP_Weapon_C|GetWeapon%20name Weapon%20to%20copy)))
    (:then_1
      (Variables|WeaponStats|SetCategory (Variables|BP_Weapon_C|GetCategory Weapon%20to%20copy)))
    (:then_2
      (Variables|WeaponStats|SetType (Variables|BP_Weapon_C|GetType Weapon%20to%20copy)))
    (:then_3
      (Variables|WeaponStats|SetCost (Variables|BP_Weapon_C|GetCost Weapon%20to%20copy)))
    (:then_4
      (Variables|WeaponStats|SetMag%20Size (Variables|BP_Weapon_C|GetMag%20Size Weapon%20to%20copy)))
    (:then_5
      (Variables|WeaponStats|SetCurrentMagValue (Variables|BP_Weapon_C|GetCurrentMagValue Weapon%20to%20copy)))
    (:then_6
      (Variables|WeaponStats|SetReload%20time (Variables|BP_Weapon_C|GetReload%20time Weapon%20to%20copy)))
    (:then_7
      (Variables|WeaponStats|SetAdditional%20ammo (Variables|BP_Weapon_C|GetAdditional%20ammo Weapon%20to%20copy)))
    (:then_8
      (Variables|WeaponStats|SetPrimary%20Ammo (Variables|BP_Weapon_C|GetPrimary%20Ammo Weapon%20to%20copy)))
    (:then_9
      (Variables|WeaponStats|SetSecondary%20Ammo (Variables|BP_Weapon_C|GetSecondary%20Ammo Weapon%20to%20copy)))))