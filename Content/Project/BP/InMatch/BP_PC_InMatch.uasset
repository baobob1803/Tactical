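; BP_PC_InMatch is the in-match player controller that gets the player's character into the level.
; On BeginPlay it passes itself to BP_GM_InMatch through GetCharacterSpawnTransform.
; Its SpawnCharacter event takes a transform, spawns a BP_Master_Character owned by the controller and possesses it.
; An Enhanced Input node for adding IMC_Main is present but unconnected, so it never runs.
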(event Custom|Spawn%20Character
  (params (Transform :type Transform))
  (bind _returnvalue (Game|SpawnActorfromClass "/Game/Project/BP/InMatch/BP_Master_Character.BP_Master_Character_C" Transform "Undefined" "MultiplyWithRoot" self 0))
  (Pawn|Possess _returnvalue))

(event EventBeginPlay
  (bind _asbp_gm_in_match (Utilities|Casting|CastToBP_GM_InMatch (Game|GetGameMode)))
  (Default|GetCharacterSpawnTransform _asbp_gm_in_match self))

(fn ConstructionScript)